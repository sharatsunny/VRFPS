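; BP_DefaultGun is a pickup gun that the first-person character holds in the right hand and fires.
; Pickup snaps it to the hand's GrenadeAttach socket with physics and collision off, while Drop detaches it and restores both.
; Both events update the character's ItemHeldInRightHand reference.
; Action spawns a FirstPersonProjectile at the muzzle with the player as instigator.
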(event EventAction
  (bind _muzzlelocation (Variables|Default|GetMuzzleLocation))
  (Game|SpawnActorfromClass "/Game/FirstPersonBP/Blueprints/FirstPersonProjectile.FirstPersonProjectile_C" (Math|Transform|MakeTransform (Transformation|GetWorldLocation _muzzlelocation) (Transformation|GetWorldRotation _muzzlelocation)) "Undefined" 0 (Variables|Default|GetPlayerRef)))

(event EventDrop
  (params (hand :type Scene%20Component%20Object%20Reference))
  (bind _gunmesh (Variables|Default|GetGunMesh))
  (Transformation|DetachFromActor "KeepWorld" "KeepWorld" "KeepWorld")
  (Physics|SetSimulatePhysics _gunmesh true)
  (Collision|SetCollisionEnabled _gunmesh "QueryAndPhysics")
  (Variables|/Game/FirstPersonBP/Blueprints/FirstPersonCharacter.FirstPersonCharacter_C|SetitemHeldInRightHand (.AsFirst%20Person%20Character (Utilities|Casting|CastToFirstPersonCharacter (Game|Player|GetPlayerPawn 0))) 0))

(event EventBeginPlay
  (bind _asfirst_person_character (Utilities|Casting|CastToFirstPersonCharacter (Game|GetPlayerCharacter 0)))
  (Variables|Default|SetPlayerRef _asfirst_person_character))

(event EventPickup
  (params (Hand :type Scene%20Component%20Object%20Reference))
  (bind _gunmesh (Variables|Default|GetGunMesh))
  (Transformation|AttachComponentToComponent Hand "GrenadeAttach" "SnapToTarget" "SnapToTarget" "KeepWorld" true)
  (Physics|SetSimulatePhysics _gunmesh false)
  (Collision|SetCollisionEnabled _gunmesh "NoCollision")
  (Variables|/Game/FirstPersonBP/Blueprints/FirstPersonCharacter.FirstPersonCharacter_C|SetitemHeldInRightHand (.AsFirst%20Person%20Character (Utilities|Casting|CastToFirstPersonCharacter (Game|Player|GetPlayerPawn 0))) self))

(fn ConstructionScript)