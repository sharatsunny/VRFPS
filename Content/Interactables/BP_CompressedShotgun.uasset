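; A pickup shotgun for the first-person character that fires a burst of projectiles.
; Pickup attaches it to the hand socket, disables mesh physics and registers it as the right-hand item; Drop reverses this.
; Action checks the player's fire-held flag, waits briefly, then spawns several ShotgunProjectiles.
; Spread comes from random spawn points within the Cone component's bounds, with every projectile sharing the Box component's rotation.
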(event EventAction
  (bind _cone (Variables|Default|GetCone))
  (bind (_origin _boxextent) (Collision|GetComponentBounds _cone))
  (if (Variables|/Game/FirstPersonBP/Blueprints/FirstPersonCharacter.FirstPersonCharacter_C|GetIsFireHeld? (Variables|Default|GetPlayerRef))
    (Utilities|FlowControl|Delay 0.5)
    (for _index (range 0 5)
      (Game|SpawnActorfromClass "/Game/FirstPersonBP/Blueprints/ShotgunProjectile.ShotgunProjectile_C" (Math|Transform|MakeTransform (Math|Random|RandomPointinBoundingBox _origin _boxextent) (Transformation|GetWorldRotation (Variables|Default|GetBox))) "AdjustIfPossibleButAlwaysSpawn" 0 (Variables|Default|GetPlayerRef)))))

(event EventDrop
  (params (hand :type Scene%20Component%20Object%20Reference))
  (bind _gunmesh (Variables|Default|GetGunMesh))
  (Transformation|DetachFromActor "KeepWorld" "KeepWorld" "KeepWorld")
  (Physics|SetSimulatePhysics _gunmesh true)
  (Collision|SetCollisionEnabled _gunmesh "QueryAndPhysics")
  (Variables|/Game/FirstPersonBP/Blueprints/FirstPersonCharacter.FirstPersonCharacter_C|SetitemHeldInRightHand (.AsFirst%20Person%20Character (Utilities|Casting|CastToFirstPersonCharacter (Game|Player|GetPlayerPawn 0))) 0))

(event EventBeginPlay
  (bind _asfirst_person_character (Utilities|Casting|CastToFirstPersonCharacter (Game|GetPlayerCharacter 0)))
  (Variables|Default|SetPlayerRef _asfirst_person_character))

(event EventPickup
  (params (Hand :type Scene%20Component%20Object%20Reference))
  (bind _gunmesh (Variables|Default|GetGunMesh))
  (Transformation|AttachComponentToComponent Hand "ShotgunAttach" "SnapToTarget" "SnapToTarget" "KeepWorld" true)
  (Physics|SetSimulatePhysics _gunmesh false)
  (Collision|SetCollisionEnabled _gunmesh "NoCollision")
  (Variables|/Game/FirstPersonBP/Blueprints/FirstPersonCharacter.FirstPersonCharacter_C|SetitemHeldInRightHand (.AsFirst%20Person%20Character (Utilities|Casting|CastToFirstPersonCharacter (Game|Player|GetPlayerPawn 0))) self))

(fn ConstructionScript)