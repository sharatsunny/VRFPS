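; Laser gun pickup that attaches to the player's hand, drops as a physics object, and fires a continuous beam while fire is held.
; A timeline calls FireLazer on each update, line tracing from the muzzle to place the beam particle's endpoints.
; Damage comes from a Box stretched by full trace length rather than impact distance, hurting overlapping "Damageable"-tagged actors every update.
; Calling Action without fire held destroys the beam and stops the timeline.
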(event Custom|FireLazer
  (bind _muzzlelocation (Variables|Default|GetMuzzleLocation))
  (bind _returnvalue (Transformation|GetWorldLocation _muzzlelocation))
  (bind _output_get (Variables|Default|SetLazerStartLocation _returnvalue))
  (bind _output_get_2 (Variables|Default|SetLazerEndLocation (+ _returnvalue (* (Math|Vector|GetForwardVector (Transformation|GetWorldRotation _muzzlelocation)) 5e+03))))
  (bind _outhit (Collision|LineTraceByChannel _output_get _output_get_2 "TraceTypeQuery2" false 0 "None"))
  (Utilities|IsValid (Variables|Default|GetLaserBeamParticle)
    (:Is%20Valid
      (Transformation|SetWorldLocation (Variables|Default|GetLaserBeamParticle) (.TraceStart (Collision|BreakHitResult _outhit)) false false))
    (:Is%20Not%20Valid
      (bind _returnvalue_2 (Effects|SpawnEmitteratLocation "/Game/ParticleEffects/P_LazerBeam.P_LazerBeam" (.TraceStart (Collision|BreakHitResult _outhit))))
      (bind _output_get_3 (Variables|Default|SetLaserBeamParticle _returnvalue_2))))
  (Class|ParticleSystemComponent|SetBeamEndPoint _output_get_3 0 (select (Math|Vector|NotEqual(Vector) (.ImpactPoint (Collision|BreakHitResult _outhit)) "0, 0, 0" 0.0001) (.ImpactPoint (Collision|BreakHitResult _outhit)) (.TraceEnd (Collision|BreakHitResult _outhit))))
  (Transformation|SetRelativeScale3D _output_get_3 "10.000000,10.000000,10.000000")
  (Transformation|SetRelativeScale3D (Variables|Default|GetBox) (Math|Vector|MakeVector (/ (Math|Vector|VectorLength (- (.TraceStart (Collision|BreakHitResult _outhit)) (.TraceEnd (Collision|BreakHitResult _outhit)))) 1.5) 0.125 0.125))
  (bind _outactors (Actor|GetAllActorswithTag "Damageable"))
  (for _array_element _outactors
    (if (Collision|IsOverlappingActor (Variables|Default|GetBox) _array_element :!class /Script/Engine.PrimitiveComponent)
      (Game|Damage|ApplyDamage _array_element 0.1 (Game|GetPlayerController 0) 0))))

(event EventAction
  (bind _laserbeamparticle (Variables|Default|GetLaserBeamParticle))
  (if (Variables|/Game/FirstPersonBP/Blueprints/FirstPersonCharacter.FirstPersonCharacter_C|GetIsFireHeld? (Variables|Default|GetPlayerRef))
    (Timeline|Update PlayFromStart
      (:Update
        (CallFunction|FireLazer)))
    (else
      (Utilities|IsValid _laserbeamparticle
        (:Is%20Valid
          (Components|DestroyComponent _laserbeamparticle)
          (Timeline|Update Stop))
        (:Is%20Not%20Valid
          (Timeline|Update Stop))))))

(event EventDrop
  (params (hand :type Scene%20Component%20Object%20Reference))
  (bind _gunmesh (Variables|Default|GetGunMesh))
  (Transformation|DetachFromActor "KeepWorld" "KeepWorld" "KeepWorld")
  (Physics|SetSimulatePhysics _gunmesh true)
  (Collision|SetCollisionEnabled _gunmesh "QueryAndPhysics")
  (Variables|/Game/FirstPersonBP/Blueprints/FirstPersonCharacter.FirstPersonCharacter_C|SetitemHeldInRightHand (.AsFirst%20Person%20Character (Utilities|Casting|CastToFirstPersonCharacter (Game|Player|GetPlayerPawn 0))) 0))

(event EventBeginPlay
  (bind _asfirst_person_character (Utilities|Casting|CastToFirstPersonCharacter (Game|GetPlayerCharacter 0)))
  (Variables|Default|SetPlayerRef _asfirst_person_character))

(event EventPickup
  (params (Hand :type Scene%20Component%20Object%20Reference))
  (bind _gunmesh (Variables|Default|GetGunMesh))
  (Transformation|AttachComponentToComponent Hand "LaserAttach" "SnapToTarget" "SnapToTarget" "KeepWorld" true)
  (Physics|SetSimulatePhysics _gunmesh false)
  (Collision|SetCollisionEnabled _gunmesh "NoCollision")
  (Variables|/Game/FirstPersonBP/Blueprints/FirstPersonCharacter.FirstPersonCharacter_C|SetitemHeldInRightHand (.AsFirst%20Person%20Character (Utilities|Casting|CastToFirstPersonCharacter (Game|Player|GetPlayerPawn 0))) self))

(fn ConstructionScript)